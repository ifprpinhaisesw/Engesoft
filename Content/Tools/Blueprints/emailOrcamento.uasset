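; Budget email Blueprint whose Negociar function decides whether a proposed price for a project is accepted.
; Proposals below 90% of the project's estimated value pass automatically, while those up to a random 10–50% above it carry a roughly 5% rejection chance.
; Anything above that margin is refused; the result sets Aceito, and acceptance overwrites Projeto.Valor with the proposal.
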(fn `negociar`
  (params (proposta :type Integer))
  (bind _returnvalue (`KismetMathLibrary.Conv_IntToDouble` proposta))
  (bind _projeto (`self.projeto`))
  (bind _valor (`/Game/Tools/Blueprints/projeto.valor` _projeto))
  (bind _returnvalue_2 (`KismetMathLibrary.Conv_IntToDouble` _valor))
  ;[1 1 1] Menor que 90% do valor estimado é aprovação automática
  (if (< _returnvalue (* (`KismetMathLibrary.Conv_IntToDouble` _valor) 0.9))
    (set `self.aceito` true)
    (set `/Game/Tools/Blueprints/projeto.valor` proposta _projeto)
    (return)
    (else
      ;[1 1 1] Dentro da margem de negociação ainda existe 5% de chance de não ser aceito
      (if (<= _returnvalue (+ _returnvalue_2 (* _returnvalue_2 (/ (`KismetMathLibrary.Conv_IntToDouble` (`KismetMathLibrary.RandomIntegerInRange` 10 50)) 100.0))))
        (if (== (`KismetMathLibrary.RandomIntegerInRange` 0 20) 0)
          (set `self.aceito` false)
          (return)
          (else
            (set `self.aceito` true)
            (set `/Game/Tools/Blueprints/projeto.valor` proposta _projeto)
            (return)))
        (else
          ;[1 1 1] Acima da margem de negociação é negado
          (set `self.aceito` false)
          (return))))))