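; Programmer attributes Blueprint with a Randomize function that generates a random programmer profile.
; A random Senior flag selects the ranges for production and salary, with seniors rolling higher in both.
; A random gender flag picks the name from a female or male name array, and burnout is rolled independently of both flags.
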(fn `randomize`
  (bind _returnvalue (`KismetMathLibrary.RandomIntegerInRange` 0 12))
  (bind _output_get (set `self.senior` (`KismetMathLibrary.RandomBool`)))
  (if _output_get
    (set `self.producao` (`KismetMathLibrary.RandomIntegerInRange` 12 15))
    (set `self.salario` (`KismetMathLibrary.RandomIntegerInRange` 9000 13000))
    (else
      (set `self.producao` (`KismetMathLibrary.RandomIntegerInRange` 1 4))
      (set `self.salario` (`KismetMathLibrary.RandomIntegerInRange` 2000 5000))))
  (bind _output_get_2 (set `self.femea` (`KismetMathLibrary.RandomBool`)))
  (if _output_get_2
    (set `self.nome` (`|GetArrayItem` (`self._nomesF`) _returnvalue))
    (else
      (set `self.nome` (`|GetArrayItem` (`self._nomesM`) _returnvalue))))
  (set `self.burnout` (`KismetMathLibrary.RandomIntegerInRange` 0 10))
  (return))