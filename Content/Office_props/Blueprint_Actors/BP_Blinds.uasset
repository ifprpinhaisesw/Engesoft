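; BP_Blinds is an office window blinds prop that is adjusted through its Rotation and CloseAmount variables.
; The construction script applies Rotation as relative yaw to a set of static mesh components, including a logo mesh, turning them together.
; It also sets the Box component's Y scale from CloseAmount.
; The event graph holds only disabled placeholder events, so the asset has no runtime logic.
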(fn `UserConstructionScript`
  (`SceneComponent.K2_SetRelativeRotation` (`self.StaticMesh6`) (`KismetMathLibrary.MakeRotator` 0.0 0.0 (`self.Rotation`)) false false)
  (`SceneComponent.K2_SetRelativeRotation` (`self.StaticMesh`) (`KismetMathLibrary.MakeRotator` 0.0 0.0 (`self.Rotation`)) false false)
  (`SceneComponent.K2_SetRelativeRotation` (`self.StaticMesh1`) (`KismetMathLibrary.MakeRotator` 0.0 0.0 (`self.Rotation`)) false false)
  (`SceneComponent.K2_SetRelativeRotation` (`self.StaticMesh2`) (`KismetMathLibrary.MakeRotator` 0.0 0.0 (`self.Rotation`)) false false)
  (`SceneComponent.K2_SetRelativeRotation` (`self.StaticMesh3`) (`KismetMathLibrary.MakeRotator` 0.0 0.0 (`self.Rotation`)) false false)
  (`SceneComponent.K2_SetRelativeRotation` (`self.StaticMesh4`) (`KismetMathLibrary.MakeRotator` 0.0 0.0 (`self.Rotation`)) false false)
  (`SceneComponent.K2_SetRelativeRotation` (`self.StaticMesh12`) (`KismetMathLibrary.MakeRotator` 0.0 0.0 (`self.Rotation`)) false false)
  (`SceneComponent.K2_SetRelativeRotation` (`self.StaticMesh5`) (`KismetMathLibrary.MakeRotator` 0.0 0.0 (`self.Rotation`)) false false)
  (`SceneComponent.K2_SetRelativeRotation` (`self.StaticMesh7`) (`KismetMathLibrary.MakeRotator` 0.0 0.0 (`self.Rotation`)) false false)
  (`SceneComponent.K2_SetRelativeRotation` (`self.StaticMesh8`) (`KismetMathLibrary.MakeRotator` 0.0 0.0 (`self.Rotation`)) false false)
  (`SceneComponent.K2_SetRelativeRotation` (`self.StaticMesh9`) (`KismetMathLibrary.MakeRotator` 0.0 0.0 (`self.Rotation`)) false false)
  (`SceneComponent.K2_SetRelativeRotation` (`self.StaticMesh10`) (`KismetMathLibrary.MakeRotator` 0.0 0.0 (`self.Rotation`)) false false)
  (`SceneComponent.K2_SetRelativeRotation` (`self.StaticMesh11`) (`KismetMathLibrary.MakeRotator` 0.0 0.0 (`self.Rotation`)) false false)
  (`SceneComponent.K2_SetRelativeRotation` (`self.SM_blinds_VB_logo_LP`) (`KismetMathLibrary.MakeRotator` 0.0 0.0 (`self.Rotation`)) false false)
  (`SceneComponent.SetRelativeScale3D` (`self.Box`) (`KismetMathLibrary.MakeVector` 1.0 (`self.CloseAmount`) 1.0)))